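; Fireball projectile actor that explodes and removes itself when its sphere overlaps a ThirdPersonCharacter.
; On authority, the overlap prints a debug string, calls PlayParticle to spawn an explosion emitter at its location, then destroys the actor after a short delay.
; The hidden-in-game call passes false, so the actor is not hidden during that delay.
; No damage is applied, and the sphere's hit event has only an empty authority switch.
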(event `self.Sphere.OnComponentBeginOverlap`
  (params (OverlappedComponent :type "PrimitiveComponent Object Reference") (OtherActor :type "Actor Object Reference") (OtherComp :type "PrimitiveComponent Object Reference") (OtherBodyIndex :type Integer) (bFromSweep :type Boolean) (SweepResult :type "HitResult Structure (by ref)"))
  (`/Engine/EditorBlueprintResources/ActorMacros.Switch Has Authority`
    (:`Authority`
      (bind _asthird_person_character (cast `/Game/ThirdPersonBP/Blueprints/ThirdPersonCharacter` OtherActor))
      (`/Engine/EditorBlueprintResources/StandardMacros.IsValid` _asthird_person_character
        (:`Is Valid`
          (`KismetSystemLibrary.PrintString` "Hello")
          (`self.PlayParticle`)
          (`self.SetActorHiddenInGame` false)
          (`KismetSystemLibrary.Delay` 0.2)
          (`self.K2_DestroyActor`))))))

(event `self.Sphere.OnComponentHit`
  (params (HitComponent :type "PrimitiveComponent Object Reference") (OtherActor :type "Actor Object Reference") (OtherComp :type "PrimitiveComponent Object Reference") (NormalImpulse :type "Vector Structure") (Hit :type "HitResult Structure (by ref)"))
  (`/Engine/EditorBlueprintResources/ActorMacros.Switch Has Authority`))

(event `PlayParticle`
  (`GameplayStatics.SpawnEmitterAtLocation` "/Game/Projectile_Stuff/FXVarietyPack/Particles/P_ky_explosion.P_ky_explosion" (`self.K2_GetActorLocation`)))

(fn `UserConstructionScript`)